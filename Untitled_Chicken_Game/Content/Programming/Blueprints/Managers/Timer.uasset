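; Day timer manager that puts a timer widget on screen, tracks seconds, minutes and total time, and drives the dinner bell and day end.
; Tick routes through server and multicast events into a one-second Delay that advances the counters.
; At DinnerBellTime it switches chickens' state, sets their blackboards to head for the coop and calls the bell event.
; Reaching DayLength sets DayOver, calls the day-over event and resets the counters.
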(event `Server Run Timer`
  ;[1 1 1] Count Seconds
  (`self.Multicast Run Timer`))

(event `Multicast Run Timer`
  ;[1 1 1] Count Seconds
  (if (not (`self.DayOver`))
    (`KismetSystemLibrary.Delay` 1.0)
    (set `self.Seconds` (+ (`self.Seconds`) 1.0))
    (set `self.TotalTime` (+ (`self.TotalTime`) 1.0))
    ;[1 1 1] Check Dinner Bell Time
    (if (<= (`self.DinnerBellTime`) (/ (`self.TotalTime`) 60.0))
      ;[1 1 1] Set GoingToCoop
      (if (`self.StateChanged`)
        ;[1 1 1] Check Day Length
        (if (== (`self.DayLength`) (/ (`self.TotalTime`) 60.0)) :!label _label
          (set `self.DayOver` true)
          (`self.DayOverEvent`)
          (`self.ResetTimer`)
          (else
            ;[1 1 1] Count Minutes
            (if (> (`self.Seconds`) 59.0) :!label _label_2
              (set `self.Minutes` (+ (`self.Minutes`) 1.0))
              (set `self.Seconds` 0.0))))
        (else
          (bind _outactors (`GameplayStatics.GetAllActorsOfClass` "/Game/Programming/Blueprints/NPCs/Chicken/ChickenAIMaster.ChickenAIMaster_C"))
          (for _array_element _outactors
            (message `/Game/Programming/Blueprints/NPCs/Chicken/IChickenAI.Change State` _array_element "NewEnumerator6")
            (bind _blackboard (`AIController.Blackboard` (`AIBlueprintHelperLibrary.GetAIController` _array_element)))
            (`BlackboardComponent.SetValueAsBool` _blackboard "GoingToCoop" true)
            (`BlackboardComponent.SetValueAsVector` _blackboard "CoopLocation" (`self.K2_GetActorLocation` (`self.CoopLocation`)))
            (set `self.StateChanged` true)
            (`self.DinnerBellRangEvent`)
            (goto _label))))
      (else
        (goto _label_2)))))

(event `self.ReceiveTick`
  (params (DeltaSeconds :type "Float (single-precision)"))
  ;[1 1 1] Count Seconds
  (`self.Server Run Timer`))

(event `self.ReceiveBeginPlay`
  ;[1 1 1] Add Timer To Screen
  (bind _returnvalue (`|CreateWidget` "/Game/Programming/Widgets/TimerWidget.TimerWidget_C"))
  (`UserWidget.AddToViewport` _returnvalue 0))

(event `ResetTimer`
  ;[1 1 1] Reset Timer
  (`self.Server Reset Timer`))

(event `Server Reset Timer`
  ;[1 1 1] Reset Timer
  (`self.Multicast Reset Timer`))

(event `Multicast Reset Timer`
  ;[1 1 1] Reset Timer
  (set `self.TotalTime` 0.0)
  (set `self.Minutes` 0.0)
  (set `self.Seconds` 0.0)
  (set `self.StateChanged` false))

(fn `UserConstructionScript`)