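; UI manager that owns the session menu widgets and toggles their visibility.
; On BeginPlay it creates the Create Session and Find Session widgets, stores them in a widget list and enables them all.
; Enabling makes each listed widget visible and adds it to the viewport, while disabling only hides them.
; A team select handler call is present but never runs.
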(event `EnableAllWidgets`
  ;[1 1 1] Set Widget Visibility
  (for _array_element (`self.WidgetList`)
    (`Widget.SetVisibility` _array_element "Visible")
    (`UserWidget.AddToViewport` _array_element 0))
  (`KismetSystemLibrary.PrintText` "Enabled all widgets"))

(event `DisableAllWidgets`
  ;[1 1 1] Set Widget Visibility
  (for _array_element (`self.WidgetList`)
    (`Widget.SetVisibility` _array_element "Hidden")))

(event `self.ReceiveBeginPlay`
  (bind _returnvalue (`|CreateWidget` "/Game/Programming/Widgets/MainMenu/Old/WB_CreateSession.WB_CreateSession_C"))
  (bind _output_get (set `self.WB_Create_Session` _returnvalue))
  (`KismetArrayLibrary.Array_Add` (`self.WidgetList`) _output_get)
  (bind _returnvalue_2 (`|CreateWidget` "/Game/Programming/Widgets/MainMenu/Old/WB_FindSession.WB_FindSession_C"))
  (bind _output_get_2 (set `self.WB_Find_Session` _returnvalue_2))
  (`KismetArrayLibrary.Array_Add` (`self.WidgetList`) _output_get_2)
  (`self.EnableAllWidgets`))

(fn `UserConstructionScript`)