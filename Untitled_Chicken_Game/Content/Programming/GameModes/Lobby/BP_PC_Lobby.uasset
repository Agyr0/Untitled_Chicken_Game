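; Player controller for the lobby, handling each player's UI, team choice, ready state and kicking.
; On local BeginPlay it shows team select, connected players and friends list widgets with UI-only mouse input.
; Ready, team and start-button changes pass through Server-prefixed events, while team selection is forwarded to BP_GM_Lobby.
; Match travel goes through the AFGI_Main game instance when allowed, and a kick opens the main menu and destroys the session.
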(event `self.ReceiveBeginPlay`
  (bind _returnvalue (`GameplayStatics.GetPlayerController` 0))
  (if (`self.IsLocalController`)
    (bind _asafgi_main (cast `/Game/Programming/GameModes/AFGI_Main` (`GameplayStatics.GetGameInstance`)))
    (set `self.Ref Server Info` _asafgi_main)
    (`/Engine/EditorBlueprintResources/StandardMacros.IsValid` (stale _returnvalue_2)
      (:`Is Valid`
        _)
      (:`Is Not Valid`
        (bind _returnvalue_2 (`|CreateWidget` "/Game/Programming/Widgets/Lobby/WB_TeamSelect.WB_TeamSelect_C" _returnvalue))
        (bind _output_get (set `self.Ref Team Select` _returnvalue_2))))
    (`UserWidget.AddToViewport` _output_get 0)
    (`/Engine/EditorBlueprintResources/StandardMacros.IsValid` (stale _returnvalue_3)
      (:`Is Valid`
        _)
      (:`Is Not Valid`
        (bind _returnvalue_3 (`|CreateWidget` "/Game/Programming/Widgets/Lobby/WB_ConnectedPlayers.WB_ConnectedPlayers_C" (`GameplayStatics.GetPlayerController` 0)))
        (bind _output_get_2 (set `self.Ref Connected Players` _returnvalue_3))))
    (`UserWidget.AddToViewport` _output_get_2 0)
    (`/Engine/EditorBlueprintResources/StandardMacros.IsValid` (stale _returnvalue_4)
      (:`Is Valid`
        _)
      (:`Is Not Valid`
        (bind _returnvalue_4 (`|CreateWidget` "/Game/Programming/Widgets/Lobby/WB_FriendsList.WB_FriendsList_C" (`GameplayStatics.GetPlayerController` 0)))
        (bind _output_get_3 (set `self.FriendsList` _returnvalue_4))))
    (`UserWidget.AddToViewport` _output_get_3 0)
    (set `PlayerController.bShowMouseCursor` true _returnvalue)
    (`WidgetBlueprintLibrary.SetInputMode_UIOnlyEx` _returnvalue null)))

(event `Server Travel`
  (if (`self.CanStart`)
    (`/Game/Programming/GameModes/AFGI_Main.Travel Server` (`self.Ref Server Info`))))

(event `Toggle Ready`
  ;[1 1 1] Tell server ready
  (bind _output_get (set `self.Player Ready` (not (`self.Player Ready`))))
  (`self.Server Ready` _output_get))

(event `SetTeam`
  (bind _output_get (set `self.IsFarmer` (not (`self.IsFarmer`))))
  (`self.ServerSetTeam` _output_get))

(event `Toggle Start Game`
  (params (Start :type "Button Object Reference (by ref)") (IsReady :type "Boolean (by ref)"))
  ;[1 1 1] Tell server ready
  (`self.Server Toggle Start Game` Start IsReady))

(event `Set Ready`
  (params (`Player Ready` :type Boolean))
  ;[1 1 1] Tell server ready
  (bind _output_get (set `self.Player Ready` `Player Ready`))
  (`self.Server Ready` _output_get))

(event `Server Toggle Start Game`
  (params (`Start Button` :type "Button Object Reference (by ref)") (IsReady :type "Boolean (by ref)"))
  ;[1 1 1] Tell server ready
  (`/Engine/EditorBlueprintResources/StandardMacros.IsValid` `Start Button`
    (:`Is Valid`
      (`Widget.SetIsEnabled` `Start Button` IsReady))))

(event `ServerSetTeam`
  (params (IsFarmer :type Boolean))
  (set `self.IsFarmer` IsFarmer))

(event `Server Ready`
  (params (ServerReady :type Boolean))
  ;[1 1 1] Tell server ready
  (set `self.Player Ready` ServerReady))

(event `Team Selected`
  (params (Team :type "/Game/Programming/GameModes/Lobby/TeamSelect Enum" :default "NewEnumerator0") (`Increase?` :type Boolean) (Controller :type "/Game/Programming/GameModes/Lobby/BP_PC_Lobby Object Reference"))
  (bind _asbp_gm_lobby (cast `/Game/Programming/GameModes/Lobby/BP_GM_Lobby` (`GameplayStatics.GetGameMode`)))
  (`/Game/Programming/GameModes/Lobby/BP_GM_Lobby.Select Team` _asbp_gm_lobby Team self `Increase?`))

(event `OC_KickPlayer`
  ;[1 1 1] Kick self
  (`GameplayStatics.OpenLevelBySoftObjectPtr` "/Game/Levels/MainMenu.MainMenu")
  (`DestroySessionCallbackProxy.DestroySession` null))

(fn `UserConstructionScript`)