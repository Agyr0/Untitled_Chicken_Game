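; Lobby HUD Blueprint that creates and displays the main menu HUD, team select and start game widgets for the owning player.
; Each widget has its own custom event that creates it, stores a reference and adds it to the viewport.
; Team select and start game widgets are also added to WidgetList, while the main menu HUD is not.
; BeginPlay is empty, so nothing in this graph triggers these events.
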(event `self.ReceiveBeginPlay`)

(event `CreateCoreHUDWidget`
  ;[1 1 1] Create Core HUD Widget
  (bind _returnvalue (`|CreateWidget` "/Game/Programming/Widgets/MainMenu/Old/WB_HUD_MainMenu.WB_HUD_MainMenu_C" (`self.GetOwningPlayerController`)))
  (bind _output_get (set `self.WB_HUD_MainMenu` _returnvalue))
  (`UserWidget.AddToViewport` _output_get 0))

(event `CreateTeamSelectWidget`
  ;[1 1 1] Create Team Select Widget
  (bind _returnvalue (`|CreateWidget` "/Game/Programming/Widgets/Lobby/WB_TeamSelect.WB_TeamSelect_C" (`self.GetOwningPlayerController`)))
  (bind _output_get (set `self.WB_Team_Select` _returnvalue))
  (`KismetArrayLibrary.Array_Add` (`self.WidgetList`) _output_get)
  (`UserWidget.AddToViewport` _output_get 0))

(event `CreateStartGameWidget`
  ;[1 1 1] Create Start Game Button
  (bind _returnvalue (`|CreateWidget` "/Game/Programming/Widgets/Lobby/Old/WB_StartGame.WB_StartGame_C" (`self.GetOwningPlayerController`)))
  (bind _output_get (set `self.WB_StartGame` _returnvalue))
  (`KismetArrayLibrary.Array_Add` (`self.WidgetList`) _output_get)
  (`UserWidget.AddToViewport` _output_get 0))

(fn `UserConstructionScript`)