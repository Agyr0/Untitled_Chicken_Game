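; Lobby game mode that tracks joining players and manages Farmer and Chicken team selection.
; PostLogin stores each controller, and SelectTeam adjusts capped team counts in BP_GS_Lobby, adding or removing player team data in the game instance by net player index.
; CheckTeamLimit returns whether a team is full and toggles its lobby select button, though returning inside the player loop means only the first player's menu updates.
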(event `self.K2_PostLogin`
  (params (NewPlayer :type "PlayerController Object Reference"))
  (`KismetArrayLibrary.Array_Add` (`self.All Players`) NewPlayer))

(event `Select Team`
  (params (Team :type "/Game/Programming/GameModes/Lobby/TeamSelect Enum" :default "NewEnumerator0") (Controller :type "/Game/Programming/GameModes/Lobby/BP_PC_Lobby Object Reference") (`Increase?` :type Boolean))
  ;[1 1 1] Handle Team Count
  (bind _asbp_gs_lobby (cast `/Game/Programming/GameModes/Lobby/BP_GS_Lobby` (`GameplayStatics.GetGameState`)))
  (if `Increase?`
    (switch `/Game/Programming/GameModes/Lobby/TeamSelect` Team
      (:`NewEnumerator1`
        (if (< (`/Game/Programming/GameModes/Lobby/BP_GS_Lobby.CurFarmers` _asbp_gs_lobby) (`/Game/Programming/GameModes/Lobby/BP_GS_Lobby.MaxFarmers` _asbp_gs_lobby))
          (`/Engine/EditorBlueprintResources/StandardMacros.IncrementInt` (`/Game/Programming/GameModes/Lobby/BP_GS_Lobby.CurFarmers` _asbp_gs_lobby)
            (:`  `
              (`/Game/Programming/GameModes/AFGI_Main.Adjust Team Data` (cast `/Game/Programming/GameModes/AFGI_Main` (`GameplayStatics.GetGameInstance`) :!pure true) Team (`AdvancedSessionsLibrary.GetNetPlayerIndex` Controller) :!label _label)))))
      (:`NewEnumerator2`
        (if (< (`/Game/Programming/GameModes/Lobby/BP_GS_Lobby.CurChickens` _asbp_gs_lobby) (`/Game/Programming/GameModes/Lobby/BP_GS_Lobby.MaxChickens` _asbp_gs_lobby))
          (`/Engine/EditorBlueprintResources/StandardMacros.IncrementInt` (`/Game/Programming/GameModes/Lobby/BP_GS_Lobby.CurChickens` _asbp_gs_lobby)
            (:`  `
              (goto _label))))))
    (else
      (switch `/Game/Programming/GameModes/Lobby/TeamSelect` Team
        (:`NewEnumerator1`
          (if (> (`/Game/Programming/GameModes/Lobby/BP_GS_Lobby.CurFarmers` _asbp_gs_lobby) 0)
            (`/Engine/EditorBlueprintResources/StandardMacros.DecrementInt` (`/Game/Programming/GameModes/Lobby/BP_GS_Lobby.CurFarmers` _asbp_gs_lobby)
              (:`  `
                (`/Game/Programming/GameModes/AFGI_Main.Remove Player Data` (cast `/Game/Programming/GameModes/AFGI_Main` (`GameplayStatics.GetGameInstance`) :!pure true) (`AdvancedSessionsLibrary.GetNetPlayerIndex` Controller) :!label _label_2)))))
        (:`NewEnumerator2`
          (if (> (`/Game/Programming/GameModes/Lobby/BP_GS_Lobby.CurChickens` _asbp_gs_lobby) 0)
            (`/Engine/EditorBlueprintResources/StandardMacros.DecrementInt` (`/Game/Programming/GameModes/Lobby/BP_GS_Lobby.CurChickens` _asbp_gs_lobby)
              (:`  `
                (goto _label_2)))))))))

(fn `CheckTeamLimit`
  (params (Team :type "/Game/Programming/GameModes/Lobby/TeamSelect Enum" :default "NewEnumerator0"))
  (returns (AtMax :type Boolean))
  (bind _asbp_gs_lobby (cast `/Game/Programming/GameModes/Lobby/BP_GS_Lobby` (`GameplayStatics.GetGameState`)))
  (for _array_element (`self.All Players`)
    (bind _asbp_pc_lobby (cast `/Game/Programming/GameModes/Lobby/BP_PC_Lobby` _array_element))
    (switch `/Game/Programming/GameModes/Lobby/TeamSelect` Team
      (:`NewEnumerator1`
        (bind _ref_wb_team_select (`/Game/Programming/Widgets/Lobby/WB_LobbyMenu.Ref WB Team Select` (`/Game/Programming/GameModes/Lobby/BP_PC_Lobby.Ref Lobby Menu` _asbp_pc_lobby)))
        (bind _returnvalue (== (`/Game/Programming/GameModes/Lobby/BP_GS_Lobby.CurFarmers` _asbp_gs_lobby) (`/Game/Programming/GameModes/Lobby/BP_GS_Lobby.MaxFarmers` _asbp_gs_lobby)))
        (`Widget.SetIsEnabled` (`/Game/Programming/Widgets/Lobby/WB_TeamSelect.Farmer_Select` _ref_wb_team_select) (not _returnvalue))
        (return _returnvalue))
      (:`NewEnumerator2`
        (bind _returnvalue_2 (== (`/Game/Programming/GameModes/Lobby/BP_GS_Lobby.CurChickens` _asbp_gs_lobby) (`/Game/Programming/GameModes/Lobby/BP_GS_Lobby.MaxChickens` _asbp_gs_lobby)))
        (`Widget.SetIsEnabled` (`/Game/Programming/Widgets/Lobby/WB_TeamSelect.Chicken_Select` _ref_wb_team_select) (not _returnvalue_2))
        (return _returnvalue_2)))))

(fn `UserConstructionScript`)