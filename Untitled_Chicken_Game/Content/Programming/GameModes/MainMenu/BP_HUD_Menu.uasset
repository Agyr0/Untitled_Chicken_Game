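; BP_HUD_Menu is the main menu HUD Blueprint, with events that create the core menu, Create Session and Find Session widgets.
; Each event creates its widget for the owning player controller, stores a reference and adds it to the viewport.
; The two session widgets are also added to WidgetList.
; BeginPlay is empty, and the in-graph calls to these creation events are disconnected.
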(event `self.ReceiveBeginPlay`)

(event `CreateMainMenuHUDWidget`
  ;[1 1 1] Create Core HUD Widget
  (bind _returnvalue (`|CreateWidget` "/Game/Programming/Widgets/MainMenu/Old/WB_HUD_MainMenu.WB_HUD_MainMenu_C" (`self.GetOwningPlayerController`)))
  (bind _output_get (set `self.WB_Core_HUD` _returnvalue))
  (`UserWidget.AddToViewport` _output_get 0))

(event `CreateCreateSessionWidget`
  ;[1 1 1] Create Create Session Widget
  (bind _returnvalue (`|CreateWidget` "/Game/Programming/Widgets/MainMenu/Old/WB_CreateSession.WB_CreateSession_C" (`self.GetOwningPlayerController`)))
  (bind _output_get (set `self.WB_Create_Session` _returnvalue))
  (`KismetArrayLibrary.Array_Add` (`self.WidgetList`) _output_get)
  (`UserWidget.AddToViewport` _output_get 0))

(event `CreateFindSessionWidget`
  ;[1 1 1] Create Find Session Widget
  (bind _returnvalue (`|CreateWidget` "/Game/Programming/Widgets/MainMenu/Old/WB_FindSession.WB_FindSession_C" (`self.GetOwningPlayerController`)))
  (bind _output_get (set `self.WB_Find_Session` _returnvalue))
  (`KismetArrayLibrary.Array_Add` (`self.WidgetList`) _output_get)
  (`UserWidget.AddToViewport` _output_get 0))

(fn `UserConstructionScript`)