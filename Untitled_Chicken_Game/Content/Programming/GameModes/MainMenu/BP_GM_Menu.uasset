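; Main menu GameMode that keeps track of connected player controllers in the AllPCs list.
; On post-login it adds the controller, has the FGI_Main game instance store the player's index, and prints a debug message.
; Controller swaps append the new controller without removing the old one.
; Logout removes the exiting controller only if it casts to BP_PC_Menu.
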(event `self.K2_PostLogin`
  (params (NewPlayer :type "PlayerController Object Reference"))
  ;[0.1545 0.1545 0.1545] Player Connection / Disconnection
  ;;[1 1 1] Events for when a player connects
  (`KismetArrayLibrary.Array_Add` (`self.All_PC's`) NewPlayer)
  (`/Game/Programming/GameModes/AFGI_Main.Store Player Index` (cast `/Game/Programming/GameModes/AFGI_Main` (`GameplayStatics.GetGameInstance`) :!pure true) NewPlayer)
  (`KismetSystemLibrary.PrintText` "Player added to list on connect"))

(event `self.K2_OnSwapPlayerControllers`
  (params (OldPC :type "PlayerController Object Reference") (NewPC :type "PlayerController Object Reference"))
  ;[0.1545 0.1545 0.1545] Player Connection / Disconnection
  ;;[1 1 1] Events for when a player connects
  (`KismetArrayLibrary.Array_Add` (`self.All_PC's`) NewPC))

(event `self.K2_OnLogout`
  (params (ExitingController :type "Controller Object Reference"))
  ;[0.1545 0.1545 0.1545] Player Connection / Disconnection
  ;;[1 1 1] Event for when player disconnects
  (bind _asbp_pc_menu (cast `/Game/Programming/GameModes/MainMenu/BP_PC_Menu` ExitingController))
  (`KismetArrayLibrary.Array_RemoveItem` (`self.All_PC's`) _asbp_pc_menu))

(fn `UserConstructionScript`)