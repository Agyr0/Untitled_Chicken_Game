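; BP_PC_Menu is the main menu player controller that shows the menu UI and relays session requests.
; On BeginPlay it caches the AFGI_Main game instance, creates and displays WB_MainMenu, shows the cursor and switches to UI-only input.
; ClientHostSession and ClientJoinSession forward to the game instance's HostSession and JoinSession.
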(event `self.ReceiveBeginPlay`
  (bind _returnvalue (`GameplayStatics.GetPlayerController` 0))
  (bind _asafgi_main (cast `/Game/Programming/GameModes/AFGI_Main` (`GameplayStatics.GetGameInstance`)))
  (set `self.Ref AFGI` _asafgi_main)
  (`/Engine/EditorBlueprintResources/StandardMacros.IsValid` (stale _returnvalue_2)
    (:`Is Valid`
      _)
    (:`Is Not Valid`
      (bind _returnvalue_2 (`|CreateWidget` "/Game/Programming/Widgets/MainMenu/WB_MainMenu.WB_MainMenu_C" (`GameplayStatics.GetPlayerController` 0)))))
  (`UserWidget.AddToViewport` _returnvalue_2 0)
  (set `PlayerController.bShowMouseCursor` true _returnvalue)
  (`WidgetBlueprintLibrary.SetInputMode_UIOnlyEx` _returnvalue _returnvalue_2))

(event `Client Host Session`
  (`/Game/Programming/GameModes/AFGI_Main.Host Session` (`self.Ref AFGI`)))

(event `Client Join Session`
  (`/Game/Programming/GameModes/AFGI_Main.Join Session` (`self.Ref AFGI`)))

(fn `UserConstructionScript`)