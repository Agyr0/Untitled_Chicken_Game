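; Player controller for the main game mode that requests the player's spawn as either a farmer or a chicken.
; SpawnPlayer runs only on the local controller and hands off to SR_SpawnPlayer, which calls the game mode's farmer or chicken spawn based on team flags.
; Players with no team default to chicken with a printed notice.
; A separate Spawn event passes an explicit team straight to the game mode.
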(event `Spawn`
  (params (Team :type "/Game/Programming/GameModes/Lobby/TeamSelect Enum" :default "NewEnumerator0"))
  (`/Game/Programming/GameModes/Game/BP_GM_Game.Spawn Player` (cast `/Game/Programming/GameModes/Game/BP_GM_Game` (`GameplayStatics.GetGameMode`) :!pure true) Team self))

(event `SpawnPlayer`
  ;[1 1 1] Spawning player
  (if (`self.IsLocalController`)
    (`self.SR_SpawnPlayer`)))

(event `SR_SpawnPlayer`
  ;[1 1 1] Spawning player
  (bind _asbp_gm_game (cast `/Game/Programming/GameModes/Game/BP_GM_Game` (`GameplayStatics.GetGameMode`)))
  (if (`self.Is_Farmer`)
    (`/Game/Programming/GameModes/Game/BP_GM_Game.SpawnFarmer` _asbp_gm_game self)
    (elif (`self.Is_Chicken`)
      (`/Game/Programming/GameModes/Game/BP_GM_Game.SpawnChicken` _asbp_gm_game self)
      (else
        (`KismetSystemLibrary.PrintText` "Player Hasnt Chosen a Team defaulting to chicken" true true (struct :`R` 1.0 :`G` 0.068686 :`A` 1.0))
        (`/Game/Programming/GameModes/Game/BP_GM_Game.SpawnChicken` _asbp_gm_game self)))))

(fn `UserConstructionScript`)