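; BP_PC_Escape is the player controller for the Escape game mode, handling input setup and the request to spawn the player.
; On possess it adds the default Enhanced Input mapping context.
; On BeginPlay, the local controller calls SR_Spawn and switches to game-only input with the cursor hidden.
; SR_Spawn looks up the controller's team in the game instance and passes it to BP_GM_Escape's SpawnPlayer.
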(event `self.ReceivePossess`
  (params (PossessedPawn :type "Pawn Object Reference"))
  (`EnhancedInputSubsystemInterface.AddMappingContext` (pcsubsystem `EnhancedInputLocalPlayerSubsystem` self) "/Game/Programming/DataAssets/Input/IMC_Default.IMC_Default" 0 (struct)))

(event `self.ReceiveBeginPlay`
  ;[1 1 1] Spawning player
  (if (`self.IsLocalPlayerController`)
    (`self.SR_Spawn`)
    (set `self.bShowMouseCursor` false)
    (`WidgetBlueprintLibrary.SetInputMode_GameOnly` self)))

(event `SR_Spawn`
  ;[1 1 1] Spawning player
  (bind _asafgi_main (cast `/Game/Programming/GameModes/AFGI_Main` (`GameplayStatics.GetGameInstance`)))
  (bind _asbp_gm_escape (cast `/Game/Programming/GameModes/Game/BP_GM_Escape` (`GameplayStatics.GetGameMode`)))
  (`/Game/Programming/GameModes/Game/BP_GM_Escape.Spawn Player` _asbp_gm_escape (`BlueprintMapLibrary.Map_Find` (`/Game/Programming/GameModes/AFGI_Main.PlayerTeamData` _asafgi_main) self) self))

(fn `UserConstructionScript`)