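; Escape game mode that manages Farmer and Chicken team slots and spawns each side's pawn.
; SelectTeam enforces team caps and updates AFGI_Main team data using player controller 0, not the passed controller.
; SpawnPlayer consumes the game instance's spawn points, retrying after a delay until found, then possesses the new pawn.
; Separate SpawnFarmer and SpawnChicken functions replace existing pawns at BP_Start_Game actors.
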(event `self.ReceiveBeginPlay`
  (bind _asafgi_main (cast `/Game/Programming/GameModes/AFGI_Main` (`GameplayStatics.GetGameInstance`)))
  (bind _output_get (set `self.As AFGI Main` _asafgi_main))
  (if (`self.HasAuthority`)
    (bind _playerteamdata (`/Game/Programming/GameModes/AFGI_Main.PlayerTeamData` _output_get))
    (bind _keys (`BlueprintMapLibrary.Map_Keys` _playerteamdata))
    (for _array_element _keys
      (`KismetSystemLibrary.PrintText` (`KismetTextLibrary.Conv_StringToText` (`KismetStringLibrary.Concat_StrStr` "Player: " (`KismetSystemLibrary.GetDisplayName` _array_element) " Team: " (`|GetEnumeratorNameAsString` (`BlueprintMapLibrary.Map_Find` _playerteamdata _array_element)) "     -GM_Escape"))))))

(event `self.K2_PostLogin`
  (params (NewPlayer :type "PlayerController Object Reference"))
  (`KismetArrayLibrary.Array_Add` (`self.All Players`) NewPlayer))

(event `Select Team`
  (params (Team :type "/Game/Programming/GameModes/Escape/TeamSelect Enum" :default "NewEnumerator0") (Controller :type "/Game/Programming/GameModes/Escape/BP_PC_Escape Object Reference") (`Increase?` :type Boolean))
  (bind _returnvalue (`GameplayStatics.GetPlayerController` 0))
  ;[1 1 1] Handle Team Count
  (if `Increase?`
    (switch `/Game/Programming/GameModes/Escape/TeamSelect` Team
      (:`NewEnumerator1`
        (if (< (`self.CurFarmers`) (`self.MaxFarmers`))
          (`/Engine/EditorBlueprintResources/StandardMacros.IncrementInt` (`self.CurFarmers`)
            (:`  `
              (`/Game/Programming/GameModes/AFGI_Main.Adjust Team Data` (cast `/Game/Programming/GameModes/AFGI_Main` (`GameplayStatics.GetGameInstance`) :!pure true) Team _returnvalue :!label _label)))))
      (:`NewEnumerator2`
        (if (< (`self.CurChickens`) (`self.MaxChickens`))
          (`/Engine/EditorBlueprintResources/StandardMacros.IncrementInt` (`self.CurChickens`)
            (:`  `
              (goto _label))))))
    (else
      (switch `/Game/Programming/GameModes/Escape/TeamSelect` Team
        (:`NewEnumerator1`
          (if (> (`self.CurFarmers`) 0)
            (`/Engine/EditorBlueprintResources/StandardMacros.DecrementInt` (`self.CurFarmers`)
              (:`  `
                (`/Game/Programming/GameModes/AFGI_Main.Remove Team Data` (cast `/Game/Programming/GameModes/AFGI_Main` (`GameplayStatics.GetGameInstance`) :!pure true) _returnvalue :!label _label_2)))))
        (:`NewEnumerator2`
          (if (> (`self.CurChickens`) 0)
            (`/Engine/EditorBlueprintResources/StandardMacros.DecrementInt` (`self.CurChickens`)
              (:`  `
                (goto _label_2)))))))))

(event `Spawn Player`
  (params (Team :type "/Game/Programming/GameModes/Escape/TeamSelect Enum" :default "NewEnumerator0") (Controller :type "/Game/Programming/GameModes/Escape/BP_PC_Escape Object Reference"))
  (bind _as_afgi_main (`self.As AFGI Main`))
  (bind _farmerspawns (`/Game/Programming/GameModes/AFGI_Main.FarmerSpawns` _as_afgi_main))
  (bind _chickenspawns (`/Game/Programming/GameModes/AFGI_Main.ChickenSpawns` _as_afgi_main))
  (bind _output (`|GetArrayItem` _farmerspawns))
  (bind _output_2 (`|GetArrayItem` _chickenspawns))
  (if (`/Game/Programming/GameModes/AFGI_Main.SpawnsFound` _as_afgi_main) :!label _label_3
    (switch `/Game/Programming/GameModes/Escape/TeamSelect` Team
      (:`NewEnumerator1`
        (bind _returnvalue (`|SpawnActorFromClass` "/Game/Programming/Blueprints/Farmer/Farmer.Farmer_C" (`self.GetTransform` _output) "Undefined" "MultiplyWithRoot" null 0.0 0.0 null))
        (`KismetArrayLibrary.Array_RemoveItem` _farmerspawns _output)
        (`Controller.Possess` Controller _returnvalue))
      (:`NewEnumerator2`
        (bind _returnvalue_2 (`|SpawnActorFromClass` "/Game/Programming/Blueprints/Chicken/Chicken_Player.Chicken_Player_C" (`self.GetTransform` _output_2) "Undefined" "MultiplyWithRoot" null null))
        (`KismetArrayLibrary.Array_RemoveItem` _chickenspawns _output_2)
        (`Controller.Possess` Controller _returnvalue_2)))
    (else
      (`KismetSystemLibrary.Delay` 0.5)
      (`/Game/Programming/GameModes/AFGI_Main.Find Spawn Points` _as_afgi_main)
      (goto _label_3))))

(fn `FindChickenStart`
  (returns (Chicken_Start_Transform :type "Transform Structure (by ref)"))
  (bind _outactors (`GameplayStatics.GetAllActorsOfClass` "/Game/Programming/Blueprints/BP_Start_Game.BP_Start_Game_C"))
  (for _array_element _outactors
    (if (`|EnumEquality` (`/Game/Programming/Blueprints/BP_Start_Game.Team` _array_element) "NewEnumerator2")
      (`KismetArrayLibrary.Array_RemoveItem` _outactors)
      (return (`self.GetTransform` (`|GetArrayItem` _outactors (`KismetMathLibrary.RandomIntegerInRange` 0 (- (`KismetArrayLibrary.Array_Length` _outactors) 1))))))))

(fn `FindFarmerStart`
  (returns (Farmer_Start_Transform :type "Transform Structure (by ref)"))
  (bind _outactors (`GameplayStatics.GetAllActorsOfClass` "/Game/Programming/Blueprints/BP_Start_Game.BP_Start_Game_C"))
  (for _array_element _outactors
    (if (`|EnumEquality` (`/Game/Programming/Blueprints/BP_Start_Game.Team` _array_element) "NewEnumerator1")
      (return (`self.GetTransform` _array_element)))))

(fn `SpawnChicken`
  (params (PlayerController :type "PlayerController Object Reference"))
  (bind _returnvalue (`Controller.K2_GetPawn` PlayerController))
  (`/Engine/EditorBlueprintResources/StandardMacros.IsValid` _returnvalue
    (:`Is Valid`
      (`self.K2_DestroyActor` _returnvalue))
    (:`Is Not Valid`
      _))
  (bind _returnvalue_2 (`|SpawnActorFromClass` "/Game/Programming/Blueprints/Chicken/Chicken_Player.Chicken_Player_C" (`self.FindChickenStart`) "Undefined" "MultiplyWithRoot" null null))
  (`Controller.Possess` PlayerController _returnvalue_2))

(fn `SpawnFarmer`
  (params (PlayerController :type "PlayerController Object Reference"))
  (bind _returnvalue (`Controller.K2_GetPawn` PlayerController))
  (`/Engine/EditorBlueprintResources/StandardMacros.IsValid` _returnvalue
    (:`Is Valid`
      (`self.K2_DestroyActor` _returnvalue))
    (:`Is Not Valid`
      _))
  (bind _returnvalue_2 (`|SpawnActorFromClass` "/Game/Programming/Blueprints/Farmer/Farmer.Farmer_C" (`self.FindFarmerStart`) "Undefined" "MultiplyWithRoot" null 0.0 0.0 null))
  (`Controller.Possess` PlayerController _returnvalue_2))

(fn `UserConstructionScript`)